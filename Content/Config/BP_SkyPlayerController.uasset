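; Player controller that sets game-and-UI input with a visible cursor at BeginPlay and routes input actions to UserProfile transactions.
; TransactionCancel ends the current transaction on the UserProfile.
; CycleUp and CycleDown share one TransactionRotate call with the same true argument, so both make an identical rotation request.
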(event `self.ReceiveBeginPlay`
  (`WidgetBlueprintLibrary.SetInputMode_GameAndUIEx` self null "DoNotLock" false true)
  (set `self.bShowMouseCursor` true))

(event `InputAction|TransactionConfirm`
  (params (Key :type "Key Structure")))

(event `InputAction|TransactionCancel`
  (params (Key :type "Key Structure"))
  (:`Pressed`
    (`UserProfile.EndTransaction` (`SkyGameMode.UserProfile` (`SkyGameMode.Get`)))))

(event `InputAction|CycleUp`
  (params (Key :type "Key Structure"))
  (:`Pressed`
    (`UserProfile.TransactionRotate` (`SkyGameMode.UserProfile` (`SkyGameMode.Get`)) true :!label _label)))

(event `InputAction|CycleDown`
  (params (Key :type "Key Structure"))
  (:`Pressed`
    (goto _label)))

(fn `UserConstructionScript`)