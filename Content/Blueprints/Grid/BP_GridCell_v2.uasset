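; BP_GridCell_v2 is the Blueprint for a grid cell that hosts units and shows highlights.
; Mouse hover and clicks on the block mesh call focus and interact functions; selectability toggles TopRoot visibility.
; Created units attach rotated by orientation, and highlight events swap materials, update the tooltip widget, which stays hidden, and set unit focus.
; Timelines for highlight rise and randomised falling cleanup are disconnected, so never run.
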(event `self.ReceiveBeginPlay`
  ;[1 1 1] Begin Play
  (`SceneComponent.SetVisibility` (`self.RootHighlights`) false true)
  (`SceneComponent.SetVisibility` (`self.RootIntents`) false true))

(event `InitialSetup`
  ;[1 0 0] Setup
)

(event `self.OnUpdatedSelectable`
  ;[1 1 1] Set selectabel
  (`SceneComponent.SetVisibility` (`self.TopRoot`) (`self.bSelectable`) true))

(event `self.UnitCreatedBP`
  (params (Unit :type "GridUnitActor Object Reference") (Orientation :type "ECellOrientation Enum" :default "None"))
  ;[1 1 1] Unit Created
  (`self.K2_SetActorRelativeRotation` Unit (select `ECellOrientation` Orientation :`East` (struct :`Yaw` 90.0) :`South` (struct :`Yaw` 180.0) :`West` (struct :`Yaw` 270.0) :!type "Rotator Structure") false false)
  (`self.K2_AttachToComponent` Unit (`self.UnitActorRoot`) "None" "SnapToTarget" "KeepRelative" "SnapToTarget" true))

(event `self.SM_BlockMesh.OnBeginCursorOver`
  (params (TouchedComponent :type "PrimitiveComponent Object Reference"))
  ;[1 1 1] Mouse Hover - Highlights
  (`self.BeginFocus`))

(event `self.SM_BlockMesh.OnEndCursorOver`
  (params (TouchedComponent :type "PrimitiveComponent Object Reference"))
  ;[1 1 1] Mouse Hover - Highlights
  (`self.EndFocus`))

(event `self.SM_BlockMesh.OnClicked`
  (params (TouchedComponent :type "PrimitiveComponent Object Reference") (ButtonPressed :type "Key Structure"))
  ;[1 1 1] Confirm CLick
  (`self.Interact`))

(event `self.BeginHighlightBP`
  (bind _highlight (`self.Highlight`))
  (bind _widget_tooltip (`self.Widget_Tooltip`))
  (bind _unitactors (`self.UnitActors`))
  ;[1 1 1] Begin Highlight
  (`self.AnimHighlightShow`)
  (`SceneComponent.SetVisibility` (`self.RootHighlights`) true true)
  (`PrimitiveComponent.SetMaterial` (`self.SM_Highlight`) 0 (select `ECellHighlight` _highlight :`Basic` "/Game/Geometry/Materials/Grid/M_GridHighlight_Basic.M_GridHighlight_Basic" :`Build` "/Game/Geometry/Materials/Grid/M_GridHighlight_Build.M_GridHighlight_Build" :`Invalid` "/Game/Geometry/Materials/Grid/M_GridHighlight_Invalid.M_GridHighlight_Invalid" :!type "MaterialInterface Object Reference"))
  ;[1 1 1] Tooltip updates
  (`SceneComponent.SetVisibility` _widget_tooltip (select `byte` _highlight :`0` false :`1` false :`2` false :`3` false) false)
  (`/Game/UI/UnitTooltips/WBP_CellUnits.UpdateUnits` (cast `/Game/UI/UnitTooltips/WBP_CellUnits` (`WidgetComponent.GetUserWidgetObject` _widget_tooltip) :!pure true) _unitactors)
  ;[1 1 1] Unit FOcus
  (for _array_element _unitactors
    (`GridUnitActor.SetFocus` _array_element true)))

(event `self.EndHighlightBP`
  ;[1 1 1] End Highlight
  (`SceneComponent.SetVisibility` (`self.RootHighlights`) false true)
  ;;[1 1 1] Tooltips
  (`SceneComponent.SetVisibility` (`self.Widget_Tooltip`) false false)
  ;[1 1 1] Unit FOcus
  (for _array_element (`self.UnitActors`)
    (`GridUnitActor.SetFocus` _array_element false)))

(event `AnimHighlightShow`
  ;[1 0 0] Anim Highlight Show
)

(event `CustomEvent_3`
  ;[1 0 0] Begin Cleanup. Set it and forget from Grid
)

(fn `UserConstructionScript`)