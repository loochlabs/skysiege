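; Grid cell actor that holds units and handles mouse hover and clicks on its block mesh.
; Hover and click call BeginHighlight, EndHighlight and Interact; highlight events show a type-specific material with a pop-up animation, toggle unit focus and show a unit tooltip for Basic highlights.
; Created units attach to the cell, rotated by orientation.
; Timelines raise the cell from a random depth on setup and sink it at randomized speed before Cleanup.
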(event `self.ReceiveBeginPlay`
  ;[1 1 1] Begin Play
  (`SceneComponent.SetVisibility` (`self.RootHighlights`) false true)
  (`SceneComponent.SetVisibility` (`self.RootIntents`) false true))

(event `InitialSetup`
  ;[1 1 1] Setup
  ;;[1 1 1] RNG Final depth
  (set `self.FinalSpawnDepth` (0.0 0.0 0.0))
  ;;[1 1 1] Initial spawn anim
  (set `self.InitialSpawnDepth` (* (0.0 0.0 1.0) (`KismetMathLibrary.RandomFloatInRange` -1000.0 -3000.0)))
  (`TimelineComponent.SetPlayRate` (`self.SpawnTimeline`) (/ 1.0 1.0))
  (bind (_direction _progress) (`Timeline|SpawnTimeline` :!via `PlayFromStart`)
    (:`Update`
      (`SceneComponent.K2_SetRelativeLocation` (`self.RootMovement`) (`KismetMathLibrary.VLerp` (`self.InitialSpawnDepth`) (`self.FinalSpawnDepth`) _progress) false false))
    (:`Finished`
      (`SceneComponent.K2_SetRelativeLocation` (`self.RootMovement`) (`self.FinalSpawnDepth`) false false))))

(event `self.OnUpdatedSelectable`
  ;[1 1 1] Set selectabel
  (`SceneComponent.SetVisibility` (`self.TopRoot`) (`self.bSelectable`) true))

(event `self.UnitCreatedBP`
  (params (Unit :type "GridUnitActor Object Reference") (Orientation :type "ECellOrientation Enum" :default "None"))
  ;[1 1 1] Unit Created
  (`self.K2_SetActorRelativeRotation` Unit (select `ECellOrientation` Orientation :`East` (struct :`Yaw` 90.0) :`South` (struct :`Yaw` 170.0) :`West` (struct :`Yaw` 270.0) :!type "Rotator Structure") false false)
  (`self.K2_AttachToComponent` Unit (`self.UnitActorRoot`) "None" "SnapToTarget" "KeepRelative" "SnapToTarget" true))

(event `self.SM_BlockMesh.OnBeginCursorOver`
  (params (TouchedComponent :type "PrimitiveComponent Object Reference"))
  ;[1 1 1] Mouse Hover - Highlights
  (`self.BeginHighlight`))

(event `self.SM_BlockMesh.OnEndCursorOver`
  (params (TouchedComponent :type "PrimitiveComponent Object Reference"))
  ;[1 1 1] Mouse Hover - Highlights
  (`self.EndHighlight`))

(event `self.SM_BlockMesh.OnClicked`
  (params (TouchedComponent :type "PrimitiveComponent Object Reference") (ButtonPressed :type "Key Structure"))
  ;[1 1 1] Confirm CLick
  (`self.Interact`))

(event `self.BeginHighlightBP`
  (bind _highlight (`self.Highlight`))
  (bind _widget_tooltip (`self.Widget_Tooltip`))
  (bind _unitactors (`self.UnitActors`))
  ;[1 1 1] Begin Highlight
  (`self.AnimHighlightShow`)
  (`SceneComponent.SetVisibility` (`self.RootHighlights`) true true)
  (`PrimitiveComponent.SetMaterial` (`self.SM_Highlight`) 0 (select `ECellHighlight` _highlight :`Basic` "/Game/Geometry/Materials/Grid/M_GridHighlight_Basic.M_GridHighlight_Basic" :`Build` "/Game/Geometry/Materials/Grid/M_GridHighlight_Build.M_GridHighlight_Build" :`Invalid` "/Game/Geometry/Materials/Grid/M_GridHighlight_Invalid.M_GridHighlight_Invalid" :!type "MaterialInterface Object Reference"))
  ;[1 1 1] Tooltip updates
  (`SceneComponent.SetVisibility` _widget_tooltip (select `ECellHighlight` _highlight :`Basic` true) false)
  (`/Game/UI/UnitTooltips/WBP_CellUnits.UpdateUnits` (cast `/Game/UI/UnitTooltips/WBP_CellUnits` (`WidgetComponent.GetUserWidgetObject` _widget_tooltip) :!pure true) _unitactors)
  ;[1 1 1] Unit FOcus
  (for _array_element _unitactors
    (`GridUnitActor.SetFocus` _array_element true)))

(event `self.EndHighlightBP`
  ;[1 1 1] End Highlight
  (`SceneComponent.SetVisibility` (`self.RootHighlights`) false true)
  ;;[1 1 1] Tooltips
  (`SceneComponent.SetVisibility` (`self.Widget_Tooltip`) false false)
  ;[1 1 1] Unit FOcus
  (for _array_element (`self.UnitActors`)
    (`GridUnitActor.SetFocus` _array_element false)))

(event `AnimHighlightShow`
  ;[1 1 1] Anim Highlight Show
  (`TimelineComponent.SetPlayRate` (`self.ShowHighlightTimeline`) (/ 1.0 0.3))
  (bind (_direction _progress) (`Timeline|ShowHighlightTimeline` :!via `PlayFromStart`)
    (:`Update`
      (`SceneComponent.K2_SetRelativeLocation` (`self.RootHighlightMesh`) (`KismetMathLibrary.VLerp` (0.0 0.0 -30.0) (0.0 0.0 0.0) _progress) false false))))

(event `self.BeginCleanupBP`
  ;[1 1 1] Begin Cleanup. Set it and forget from Grid
  (if (not (`self.CleanupActive`))
    (set `self.CleanupActive` true)
    (`TimelineComponent.SetPlayRate` (`self.CleanupTimeline`) (/ 1.0 (`KismetMathLibrary.RandomFloatInRange` 4.0 6.0)))
    (bind (_direction _progress) (`Timeline|CleanupTimeline` :!via `PlayFromStart`)
      (:`Update`
        (`SceneComponent.K2_SetRelativeLocation` (`self.RootMovement`) (`KismetMathLibrary.VLerp` (0.0 0.0 0.0) (0.0 0.0 -3000.0) _progress) false false))
      (:`Finished`
        (`self.Cleanup`)))))

(fn `UserConstructionScript`)