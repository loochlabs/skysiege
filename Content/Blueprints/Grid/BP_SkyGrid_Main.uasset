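; BP_SkyGrid_Main is a grid actor that lays out cells and serves as the macro view target.
; CreateCellBP snaps a given cell to SceneRoot, then sets its relative location from Row and Col times BlockSpacing, offset by the root's relative location.
; SetViewtoMacroBP briefly blends the first player controller's view to the grid actor itself.
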(event `self.CreateCellBP`
  (params (cell :type "GridCellActor Object Reference"))
  (bind _blockspacing (`self.BlockSpacing`))
  ;[1 1 1] Create Cell
  (`self.K2_AttachToComponent` cell (`self.SceneRoot`) "None" "SnapToTarget" "SnapToTarget" "SnapToTarget" true)
  (`self.K2_SetActorRelativeLocation` cell (+ (`KismetMathLibrary.MakeVector` (* (`GridCellActor.Row` cell) _blockspacing) (* (`GridCellActor.Col` cell) _blockspacing)) (`SceneComponent.RelativeLocation` (`self.SceneRoot`))) false false))

(event `self.SetViewToMacroBP`
  ;[1 1 1] SetCameraToMacro View
  (`PlayerController.SetViewTargetWithBlend` (`GameplayStatics.GetPlayerController` 0) self 0.15 "VTBlend_Linear" 0.0 false))

(fn `UserConstructionScript`)