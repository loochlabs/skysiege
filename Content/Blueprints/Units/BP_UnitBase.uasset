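; Base actor for a grid-placed battle unit, drawing its footprint, icon and bonus cells from its unit template.
; Construction maps coordinates to cell and bonus meshes; setup shows occupied cells, scales the icon to fit, and textures bonus planes by gameplay tag.
; Grid orientation rotates the geometry, and focus toggles the bonus cells.
; HP, fatigue and food events forward to the unit's actions widget; clearing plays a delayed flip before destroying the actor.
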(event `SetOrientationRotation`
  ;[1 1 1] Orientation Rotation
  (`SceneComponent.K2_SetRelativeRotation` (`self.GeometryRoot`) (select `ECellOrientation` (`self.GridOrientation`) :`North` (struct :`Yaw` 180.0) :`East` (struct :`Yaw` 270.0) :`West` (struct :`Yaw` 90.0) :!type "Rotator Structure") false false :!label _label))

(event `self.OnUpdatedOrientation`
  ;[1 1 1] Orientation Rotation
  (goto _label))

(event `self.OnSetupComplete`
  (bind (_unitclass _shopcost _shopweight _gridshape _unittags _tagsrequiredtobuild _tagsblockingbuild _unitstats _bonusconfig _tooltipname _icon) (break `UnitTemplate` (`SkyGameMode.GetUnitTemplate` (`SkyGameMode.Get`) (`self.UnitKey`))))
  ;[1 1 1] Setup Complete
  (`self.SetOrientationRotation`)
  (bind _returnvalue (`PrimitiveComponent.CreateDynamicMaterialInstance` (`self.SM_UnitIcon`) 0 "/Game/Blueprints/Units/M_UnitIcon.M_UnitIcon" "None"))
  (`MaterialInstanceDynamic.SetTextureParameterValue` _returnvalue "IconTexture" _icon)
  ;[1 1 1] GridSize setup
  (bind _values (`BlueprintMapLibrary.Map_Values` (`self.GridShapeCells`)))
  (for _array_element _values
    (`SceneComponent.SetVisibility` _array_element false false))
  (for _array_element_2 _gridshape
    (bind (_row _col) (break `Coordinates` _array_element_2))
    (set `self.IconGridSize` (`KismetMathLibrary.Max` _col (`KismetMathLibrary.Max` _row (`self.IconGridSize`))))
    (bind (_value _returnvalue_2) (`BlueprintMapLibrary.Map_Find` (`self.GridShapeCells`) _array_element_2))
    (if _returnvalue_2
      (`SceneComponent.SetVisibility` _value true false)))
  (`SceneComponent.SetRelativeScale3D` (`self.Root_Icon`) (* (+ (`self.IconGridSize`) 1) (1.0 1.0 1.0)))
  ;[1 1 1] Bonuses
  (`SceneComponent.SetVisibility` (`self.Root_Bonuses`) false true)
  (for _array_element_3 _bonusconfig
    (bind (_coords _tagsrequiredtoapply) (break `UnitBonusConfig` _array_element_3))
    (for _array_element_4 _coords
      (bind _returnvalue_3 (`PrimitiveComponent.CreateDynamicMaterialInstance` (`BlueprintMapLibrary.Map_Find` (`self.BonusCells`) _array_element_4) 0 "/Game/Blueprints/Units/M_UnitBonus.M_UnitBonus" "None"))
      (`MaterialInstanceDynamic.SetTextureParameterValue` _returnvalue_3 "IconTexture" (`BlueprintMapLibrary.Map_Find` (`self.BonusTextures`) (`|GetArrayItem` (`BlueprintGameplayTagLibrary.BreakGameplayTagContainer` _tagsrequiredtoapply))))
      (`MaterialInstanceDynamic.SetScalarParameterValue` _returnvalue_3 "ColorStrength" (`self.UnitTextureColorStrength`)))))

(event `ClearBP_1`
  (params (delay :type "Float (single-precision)"))
  ;[1 1 1] Clear
  (`KismetSystemLibrary.Delay` delay)
  (`TimelineComponent.SetPlayRate` (`self.ClearTimeline`) (/ 1.0 0.5))
  (bind (_direction _rotationprogress) (`Timeline|ClearTimeline` :!via `PlayFromStart`)
    (:`Update`
      (`SceneComponent.K2_SetRelativeRotation` (`self.RootTopMeshes`) (`KismetMathLibrary.RLerp` (struct) (struct :`Pitch` 180.0) _rotationprogress true) false false))
    (:`Finished`
      (`self.K2_DestroyActor`))))

(event `self.OnBattleEvent`
  (params (Event :type "BattleEvent Structure (by ref)"))
  ;[1 1 1] On Battle
  (switch `EBattleEventID` (`.EventID` (break `BattleEvent` Event))
    (:`AddHP`
      _)
    (:`RemoveHP`
      _)
    (:`FatigueDamage`
      _)
    (:`AddFood`
      _)
    (:`NotEnoughFood`
      _))
  (`/Game/UI/Battle/WBP_UnitActions.HandleBattleEvent` (cast `/Game/UI/Battle/WBP_UnitActions` (`WidgetComponent.GetUserWidgetObject` (`self.Widget_BattleEvent`)) :!pure true) Event))

(event `self.OnUpdatedFocus`
  (params (bFocused :type Boolean))
  ;[1 1 1] Focus
  (for _array_element (`.BonusConfig` (break `UnitTemplate` (`SkyGameMode.GetUnitTemplate` (`SkyGameMode.Get`) (`self.UnitKey`))))
    (for _array_element_2 (`.Coords` (break `UnitBonusConfig` _array_element))
      (`SceneComponent.SetVisibility` (`BlueprintMapLibrary.Map_Find` (`self.BonusCells`) _array_element_2) bFocused false))))

(fn `AddBonusMesh`
  (params (Row :type Integer) (Col :type Integer) (Mesh :type "StaticMeshComponent Object Reference"))
  (`BlueprintMapLibrary.Map_Add` (`self.BonusCells`) (make `Coordinates` Row Col) Mesh))

(fn `UserConstructionScript`
  (bind _gridshapecells (`self.GridShapeCells`))
  (`|ExecutionSequence`
    (:`then_0`
      (`BlueprintMapLibrary.Map_Clear` _gridshapecells)
      (`BlueprintMapLibrary.Map_Add` _gridshapecells (make `Coordinates` 0 0) (`self.SM_Cell_0x0`))
      (`BlueprintMapLibrary.Map_Add` _gridshapecells (make `Coordinates` 0 1) (`self.SM_Cell_0x1`))
      (`BlueprintMapLibrary.Map_Add` _gridshapecells (make `Coordinates` 0 2) (`self.SM_Cell_0x2`))
      (`BlueprintMapLibrary.Map_Add` _gridshapecells (make `Coordinates` 0 3) (`self.SM_Cell_0x3`))
      (`BlueprintMapLibrary.Map_Add` _gridshapecells (make `Coordinates` 1 0) (`self.SM_Cell_1x0`))
      (`BlueprintMapLibrary.Map_Add` _gridshapecells (make `Coordinates` 1 1) (`self.SM_Cell_1x1`))
      (`BlueprintMapLibrary.Map_Add` _gridshapecells (make `Coordinates` 1 2) (`self.SM_Cell_1x2`))
      (`BlueprintMapLibrary.Map_Add` _gridshapecells (make `Coordinates` 1 3) (`self.SM_Cell_1x3`))
      (`BlueprintMapLibrary.Map_Add` _gridshapecells (make `Coordinates` 2 0) (`self.SM_Cell_2x0`))
      (`BlueprintMapLibrary.Map_Add` _gridshapecells (make `Coordinates` 2 1) (`self.SM_Cell_2x1`))
      (`BlueprintMapLibrary.Map_Add` _gridshapecells (make `Coordinates` 2 2) (`self.SM_Cell_2x2`))
      (`BlueprintMapLibrary.Map_Add` _gridshapecells (make `Coordinates` 2 3) (`self.SM_Cell_2x3`))
      (`BlueprintMapLibrary.Map_Add` _gridshapecells (make `Coordinates` 3 0) (`self.SM_Cell_3x0`))
      (`BlueprintMapLibrary.Map_Add` _gridshapecells (make `Coordinates` 3 1) (`self.SM_Cell_3x1`))
      (`BlueprintMapLibrary.Map_Add` _gridshapecells (make `Coordinates` 3 2) (`self.SM_Cell_3x2`))
      (`BlueprintMapLibrary.Map_Add` _gridshapecells (make `Coordinates` 3 3) (`self.SM_Cell_3x3`)))
    (:`then_1`
      (`BlueprintMapLibrary.Map_Clear` (`self.BonusCells`))
      (`self.AddBonusMesh` 0 0 (`self.Plane_Bonus_0x0`))
      (`self.AddBonusMesh` 0 1 (`self.Plane_Bonus_0x1`))
      (`self.AddBonusMesh` 0 2 (`self.Plane_Bonus_0x2`))
      (`self.AddBonusMesh` 0 3 (`self.Plane_Bonus_0x3`))
      (`self.AddBonusMesh` 1 0 (`self.Plane_Bonus_1x0`))
      (`self.AddBonusMesh` 1 1 (`self.Plane_Bonus_1x1`))
      (`self.AddBonusMesh` 1 2 (`self.Plane_Bonus_1x2`))
      (`self.AddBonusMesh` 1 3 (`self.Plane_Bonus_1x3`))
      (`self.AddBonusMesh` 2 0 (`self.Plane_Bonus_2x0`))
      (`self.AddBonusMesh` 2 1 (`self.Plane_Bonus_2x1`))
      (`self.AddBonusMesh` 2 2 (`self.Plane_Bonus_2x2`))
      (`self.AddBonusMesh` 2 3 (`self.Plane_Bonus_2x3`))
      (`self.AddBonusMesh` 3 0 (`self.Plane_Bonus_3x0`))
      (`self.AddBonusMesh` 3 1 (`self.Plane_Bonus_3x1`))
      (`self.AddBonusMesh` 3 2 (`self.Plane_Bonus_3x2`))
      (`self.AddBonusMesh` 3 3 (`self.Plane_Bonus_3x3`))
      (`self.AddBonusMesh` 0 -1 (`self.Plane_Bonus_0xn1`))
      (`self.AddBonusMesh` 0 -2 (`self.Plane_Bonus_0xn2`))
      (`self.AddBonusMesh` 0 -3 (`self.Plane_Bonus_0xn3`))
      (`self.AddBonusMesh` 1 -1 (`self.Plane_Bonus_1xn1`))
      (`self.AddBonusMesh` 1 -2 (`self.Plane_Bonus_1xn2`))
      (`self.AddBonusMesh` 1 -3 (`self.Plane_Bonus_1xn3`))
      (`self.AddBonusMesh` 2 -1 (`self.Plane_Bonus_2xn1`))
      (`self.AddBonusMesh` 2 -2 (`self.Plane_Bonus_2xn2`))
      (`self.AddBonusMesh` 2 -3 (`self.Plane_Bonus_2xn3`))
      (`self.AddBonusMesh` 3 -1 (`self.Plane_Bonus_3xn1`))
      (`self.AddBonusMesh` 3 -2 (`self.Plane_Bonus_3xn2`))
      (`self.AddBonusMesh` 3 -3 (`self.Plane_Bonus_3xn3`))
      (`self.AddBonusMesh` -1 0 (`self.Plane_Bonus_n1x0`))
      (`self.AddBonusMesh` -1 1 (`self.Plane_Bonus_n1x1`))
      (`self.AddBonusMesh` -1 2 (`self.Plane_Bonus_n1x2`))
      (`self.AddBonusMesh` -1 3 (`self.Plane_Bonus_n1x3`))
      (`self.AddBonusMesh` -2 0 (`self.Plane_Bonus_n2x0`))
      (`self.AddBonusMesh` -2 1 (`self.Plane_Bonus_n2x1`))
      (`self.AddBonusMesh` -2 2 (`self.Plane_Bonus_n2x2`))
      (`self.AddBonusMesh` -2 3 (`self.Plane_Bonus_n2x3`))
      (`self.AddBonusMesh` -3 0 (`self.Plane_Bonus_n3x0`))
      (`self.AddBonusMesh` -3 1 (`self.Plane_Bonus_n3x1`))
      (`self.AddBonusMesh` -3 2 (`self.Plane_Bonus_n3x2`))
      (`self.AddBonusMesh` -3 3 (`self.Plane_Bonus_n3x3`))
      (`self.AddBonusMesh` -1 -1 (`self.Plane_Bonus_n1xn1`))
      (`self.AddBonusMesh` -1 -2 (`self.Plane_Bonus_n1xn2`))
      (`self.AddBonusMesh` -1 -3 (`self.Plane_Bonus_n1xn3`))
      (`self.AddBonusMesh` -2 -1 (`self.Plane_Bonus_n2xn1`))
      (`self.AddBonusMesh` -2 -2 (`self.Plane_Bonus_n2xn2`))
      (`self.AddBonusMesh` -2 -3 (`self.Plane_Bonus_n2xn3`))
      (`self.AddBonusMesh` -3 -1 (`self.Plane_Bonus_n3xn1`))
      (`self.AddBonusMesh` -3 -2 (`self.Plane_Bonus_n3xn2`))
      (`self.AddBonusMesh` -3 -3 (`self.Plane_Bonus_n3xn3`)))))