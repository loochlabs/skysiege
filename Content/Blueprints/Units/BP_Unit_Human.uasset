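; Human battle unit Blueprint that supplies icon animations and status-upgrade visuals.
; Battle events call the parent handler, then play timelines that pulse the icon's scale, or rotate it for missed actions.
; On tag updates, strength and feeding status tags map to three tiers of arm and head attachments.
; Each attachment sets texture and tier tint parameters on the unit material and spawns confetti.
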(event `self.OnBattleEvent`
  (params (Event :type "BattleEvent Structure (by ref)"))
  (`parent.OnBattleEvent` Event)
  (switch `EBattleEventID` (`.EventID` (break `BattleEvent` Event))
    (:`None`
      (bind (_direction _alpha) (`Timeline|BattleEventTimeline` :!via `PlayFromStart` :!label _label)
        (:`Update`
          (`SceneComponent.SetRelativeScale3D` (`self.Root_Icon`) (`KismetMathLibrary.VLerp` (1.0 1.0 1.0) (1.5 1.5 1.5) _alpha)))
        (:`Finished`
          (`SceneComponent.SetRelativeScale3D` (`self.Root_Icon`) (1.0 1.0 1.0)))))
    (:`ActionMissed`
      (bind (_direction_2 _alpha_2) (`Timeline|MissedTimeline` :!via `PlayFromStart`)
        (:`Update`
          (`SceneComponent.K2_SetRelativeRotation` (`self.RootAnim_Icon`) (`KismetMathLibrary.RLerp` (struct :`Pitch` -20.0) (struct :`Pitch` 20.0) _alpha_2 true) false false))
        (:`Finished`
          (`SceneComponent.K2_SetRelativeRotation` :`self` (`self.RootAnim_Icon`)))))
    (:`AddMaxHP`
      (goto _label :!via `PlayFromStart`))
    (:`RemoveMaxHP`
      (goto _label :!via `PlayFromStart`))
    (:`AddHP`
      (goto _label :!via `PlayFromStart`))
    (:`RemoveHP`
      (goto _label :!via `PlayFromStart`))
    (:`FatigueDamage`
      (goto _label :!via `PlayFromStart`))
    (:`AddFood`
      (goto _label :!via `PlayFromStart`))
    (:`RemoveFood`
      (goto _label :!via `PlayFromStart`))
    (:`NotEnoughFood`
      (goto _label :!via `PlayFromStart`))
    (:`MatchWinner`
      (goto _label :!via `PlayFromStart`))))

(event `ShowUpgradeVFX`
  (`NiagaraFunctionLibrary.SpawnSystemAttached` "/Game/VFX/NS_Confetti.NS_Confetti" (`self.Root_Icon`) "None" (0.0 0.0 0.0) (struct) "KeepRelativeOffset"))

(event `SetAttachment`
  (params (Level :type Integer) (AttachmentBoolName :type Name) (AttachmentIconName :type Name) (AttachmentIconTexture :type "Texture Object Reference") (AttachmentTintName :type Name))
  (bind _unitmaterial (`self.UnitMaterial`))
  (`MaterialInstanceDynamic.SetScalarParameterValue` _unitmaterial AttachmentBoolName 1.0)
  (`MaterialInstanceDynamic.SetTextureParameterValue` _unitmaterial AttachmentIconName AttachmentIconTexture)
  (`MaterialInstanceDynamic.SetVectorParameterValue` _unitmaterial AttachmentTintName (select `int` Level :`0` (struct :`R` 0.283149 :`G` 0.708376 :`B` 0.141263 :`A` 1.0) :`1` (struct :`R` 0.074214 :`G` 0.327778 :`B` 0.791298 :`A` 1.0) :`2` (struct :`R` 0.391573 :`G` 0.23074 :`B` 0.89627 :`A` 1.0) :!type "LinearColor Structure"))
  (`self.ShowUpgradeVFX`))

(event `SetAttachmentArm`
  (params (Level :type Integer))
  (`self.SetAttachment` Level "UseAttachmentArms" "IconArms" "/Game/Art/Textures/humans/attachments/attachment_arms_1x1_v0.attachment_arms_1x1_v0" "IconArmsTint"))

(event `SetAttachmentHead`
  (params (Level :type Integer))
  (`self.SetAttachment` Level "UseAttachmentHead" "IconHead" "/Game/Art/Textures/humans/attachments/attachment_apple_helmet_1x1_v0.attachment_apple_helmet_1x1_v0" "IconTintHead"))

(event `self.OnUpdatedTags`
  (for _array_element (`BlueprintGameplayTagLibrary.BreakGameplayTagContainer` (`self.UnitTags`))
    (`|ExecutionSequence`
      (:`then_0`
        ;[1 1 1] Strong / Bulky / Meat Head
        (if (`BlueprintGameplayTagLibrary.HasTag` (`BlueprintGameplayTagLibrary.MakeLiteralGameplayTagContainer` (struct :`GameplayTags` (struct :`(TagName` "Unit.Status.Strong")))) _array_element)
          (`self.SetAttachmentArm` 0)))
      (:`then_1`
        (if (`BlueprintGameplayTagLibrary.HasTag` (`BlueprintGameplayTagLibrary.MakeLiteralGameplayTagContainer` (struct :`GameplayTags` (struct :`(TagName` "Unit.Status.Bulky")))) _array_element)
          (`self.SetAttachmentArm` 1)))
      (:`then_2`
        (if (`BlueprintGameplayTagLibrary.HasTag` (`BlueprintGameplayTagLibrary.MakeLiteralGameplayTagContainer` (struct :`GameplayTags` (struct :`(TagName` "Unit.Status.MeatHead")))) _array_element)
          (`self.SetAttachmentArm` 2)))
      (:`then_3`
        ;[1 1 1] Fed / Overrate / Glutton
        (if (`BlueprintGameplayTagLibrary.HasTag` (`BlueprintGameplayTagLibrary.MakeLiteralGameplayTagContainer` (struct :`GameplayTags` (struct :`(TagName` "Unit.Status.Fed")))) _array_element)
          (`self.SetAttachmentHead` 0))
        (if (`BlueprintGameplayTagLibrary.HasTag` (`BlueprintGameplayTagLibrary.MakeLiteralGameplayTagContainer` (struct :`GameplayTags` (struct :`(TagName` "Unit.Status.Overate")))) _array_element)
          (`self.SetAttachmentHead` 1))
        (if (`BlueprintGameplayTagLibrary.HasTag` (`BlueprintGameplayTagLibrary.MakeLiteralGameplayTagContainer` (struct :`GameplayTags` (struct :`(TagName` "Unit.Status.Glutton")))) _array_element)
          (`self.SetAttachmentHead` 2))))))

(fn `UserConstructionScript`)