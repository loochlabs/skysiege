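; BP_Shop is a shop that lets the player sell the active transaction by clicking its cube mesh.
; It listens for transaction updates on the UserProfile, showing the sell price widget and refreshing its price only while a transaction is active.
; A click asks the UserProfile to attempt the sale, and a positive result is passed to a second widget component that displays the sale.
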(event `self.ReceiveBeginPlay`
  (add `UserProfile.OnUpdatedTransaction` (`SkyGameMode.UserProfile` (`SkyGameMode.Get`)) (delegate `OnUpdatedTransaction_Event`)))

(event `OnUpdatedTransaction_Event`
  (bind _userprofile (`SkyGameMode.UserProfile` (`SkyGameMode.Get`)))
  (bind _returnvalue (`UserProfile.IsTransactionActive` _userprofile))
  (`SceneComponent.SetVisibility` (`self.Widget_SellPrice`) _returnvalue false)
  (if _returnvalue
    (`/Game/Blueprints/shop/WBP_ShopSellPrice.UpdatePrice` (cast `/Game/Blueprints/shop/WBP_ShopSellPrice` (`WidgetComponent.GetUserWidgetObject` (`self.Widget_SellPrice`)) :!pure true) (`UserProfile.GetTransactionSellPrice` _userprofile))))

(event `self.SM_Cube.OnClicked`
  (params (TouchedComponent :type "PrimitiveComponent Object Reference") (ButtonPressed :type "Key Structure"))
  (bind _returnvalue (`UserProfile.TryToSell` (`SkyGameMode.UserProfile` (`SkyGameMode.Get`))))
  (if (> _returnvalue 0)
    (`/Game/Blueprints/shop/WBP_ShopSell.DisplaySell` (cast `/Game/Blueprints/shop/WBP_ShopSell` (`WidgetComponent.GetUserWidgetObject` (`self.Widget_Sell`)) :!pure true) _returnvalue)))

(fn `UserConstructionScript`)